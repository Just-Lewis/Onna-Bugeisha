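; Trigger_Object is a component that makes its owner one element of a multi-part trigger tracked by a receiver actor.
; On BeginPlay or receiver assignment, it registers with that actor's Trigger_Reciever component, printing the owner's name and a warning if none is valid.
; SetComplete stores the completion flag, decrements the receiver's remaining count regardless of that flag's value, and calls FinishCheck.
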(event Custom|AddToElements
  (bind _triggerreciever (Variables|Default|GetTriggerReciever))
  (if (Utilities|IsValid _triggerreciever)
    (Default|AddtoNumberOfElements (Actor|GetComponentbyClass _triggerreciever "/Game/OB_Content/Blueprints/Functions/Trigger_Reciever.Trigger_Reciever_C"))
    (else
      (Development|PrintString (Utilities|GetObjectName (Components|GetOwner)))
      (Development|PrintString "Missing trigger reciever"))))

(event EventBeginPlay
  (bind _triggerreciever (Variables|Default|GetTriggerReciever))
  (if (Utilities|IsValid _triggerreciever)
    (Default|AddtoNumberOfElements (Actor|GetComponentbyClass _triggerreciever "/Game/OB_Content/Blueprints/Functions/Trigger_Reciever.Trigger_Reciever_C"))
    (else
      (Development|PrintString (Utilities|GetObjectName (Components|GetOwner)))
      (Development|PrintString "Missing trigger reciever"))))

(fn SetComplete
  (params (Complete :type Boolean))
  (bind _triggerreciever (Variables|Default|GetTriggerReciever))
  (bind _returnvalue (Actor|GetComponentbyClass _triggerreciever "/Game/OB_Content/Blueprints/Functions/Trigger_Reciever.Trigger_Reciever_C"))
  (Variables|Default|SetComplete Complete)
  (Development|PrintString "This one is compreeet")
  (Variables|/Game/OB_Content/Blueprints/Functions/Trigger_Reciever.Trigger_Reciever_C|SetNumberOfElementsToComplete _returnvalue (+ (Variables|/Game/OB_Content/Blueprints/Functions/Trigger_Reciever.Trigger_Reciever_C|GetNumberOfElementsToComplete _returnvalue) -1))
  (Default|FinishCheck _returnvalue))

(fn SetReciever
  (params (TriggerReciever :type Actor%20Object%20Reference))
  (Variables|Default|SetTriggerReciever TriggerReciever)
  (CallFunction|AddtoElements))