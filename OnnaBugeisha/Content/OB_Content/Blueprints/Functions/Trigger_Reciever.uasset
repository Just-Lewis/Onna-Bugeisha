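; Trigger_Reciever is a component that tracks how many trigger elements remain to be completed for its owning actor.
; AddToNumberOfElements increments the remaining count, while nothing in this file decrements it.
; When the count is below one, FinishCheck prints it, calls Activate on the owner's StaticMeshComponent and sets AllComplete.
; An alternative loop checking each Trigger_Object's Complete flag is left disconnected.
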(fn FinishCheck
  (bind _numberofelementstocomplete (Variables|Default|GetNumberOfElementsToComplete))
  (if (< _numberofelementstocomplete 1)
    (Development|PrintString (Utilities|String|ToString(Integer) _numberofelementstocomplete))
    (Components|Activation|Activate (Actor|GetComponentbyClass (Components|GetOwner) "/Script/Engine.StaticMeshComponent") false)
    (Variables|Default|SetAllComplete true)))

(fn AddtoNumberOfElements
  (Variables|Default|SetNumberOfElementsToComplete (+ (Variables|Default|GetNumberOfElementsToComplete) 1)))