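; YenFragment3 is a puzzle piece actor that completes a trigger when it collides with another Yen fragment.
; On hit by a "YenFrag"-tagged actor, it snaps that actor to its mesh's CentreSocket, passes the attach result to TriggerObject, then destroys itself.
; BeginPlay links TriggerObject to its receiver and records the start height.
; Tick returns the piece to that height if it falls too far below it.
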(event EventBeginPlay
  (Default|SetReciever (Variables|Default|GetTrigger_Object) (Variables|Default|GetTriggerReciever))
  (Variables|Default|SetStartHeight (.Z (Math|Vector|BreakVector (Transformation|GetActorLocation)))))

(event Collision|EventActorBeginOverlap
  (params (OtherActor :type Actor%20Object%20Reference)))

(event EventTick
  (params (DeltaSeconds :type Float%20%28single-precision%29))
  (bind _returnvalue (Transformation|GetActorLocation))
  (bind _startheight (Variables|Default|GetStartHeight))
  (bind (_x _y _z) (Math|Vector|BreakVector _returnvalue))
  (if (< _z (+ _startheight -1e+03))
    (Transformation|SetActorLocation (Math|Vector|MakeVector _x _y _startheight) false false)))

(event Collision|EventHit
  (params (MyComp :type Primitive%20Component%20Object%20Reference) (Other :type Actor%20Object%20Reference) (OtherComp :type Primitive%20Component%20Object%20Reference) (bSelfMoved :type Boolean) (HitLocation :type Vector :default "0, 0, 0") (HitNormal :type Vector :default "0, 0, 0") (NormalImpulse :type Vector :default "0, 0, 0") (Hit :type Hit%20Result%20Structure%20%28by%20ref%29))
  (if (Actor|ActorHasTag Other "YenFrag")
    (bind _returnvalue (Transformation|AttachComponentToComponent (Variables|/Script/Engine.Actor|GetRootComponent Other) (Variables|Debug|GetStaticMeshComponent) "CentreSocket" "SnapToTarget" "SnapToTarget" "SnapToTarget" true))
    (Default|SetComplete (Variables|Default|GetTrigger_Object) _returnvalue)
    (Actor|DestroyActor)
    (Transformation|AddActorWorldOffset "0, 0,20.000000")))

(fn ConstructionScript)