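; YenFragment1 is a puzzle piece Blueprint that completes when it hits an actor tagged YenFrag.
; On hit, it attaches that actor's root to its StaticMeshComponent at CentreSocket, passes the result to TriggerObject's SetComplete, then destroys itself.
; BeginPlay hands TriggerReciever to TriggerObject and records the start height.
; Tick moves the piece to world origin, rather than its start position, if it falls far below that height.
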(event EventBeginPlay
  (Default|SetReciever (Variables|Default|GetTrigger_Object) (Variables|Default|GetTriggerReciever))
  (Variables|Default|SetStartHeight (.Z (Math|Vector|BreakVector (Transformation|GetActorLocation)))))

(event Collision|EventActorBeginOverlap
  (params (OtherActor :type Actor%20Object%20Reference)))

(event EventTick
  (params (DeltaSeconds :type Float%20%28single-precision%29))
  (if (< (.Z (Math|Vector|BreakVector (Transformation|GetActorLocation))) (+ (Variables|Default|GetStartHeight) -1e+03))
    (Transformation|SetActorLocation "0, 0, 0" false false)))

(event Collision|EventHit
  (params (MyComp :type Primitive%20Component%20Object%20Reference) (Other :type Actor%20Object%20Reference) (OtherComp :type Primitive%20Component%20Object%20Reference) (bSelfMoved :type Boolean) (HitLocation :type Vector :default "0, 0, 0") (HitNormal :type Vector :default "0, 0, 0") (NormalImpulse :type Vector :default "0, 0, 0") (Hit :type Hit%20Result%20Structure%20%28by%20ref%29))
  (if (Actor|ActorHasTag Other "YenFrag")
    (bind _returnvalue (Transformation|AttachComponentToComponent (Variables|/Script/Engine.Actor|GetRootComponent Other) (Variables|Debug|GetStaticMeshComponent) "CentreSocket" "SnapToTarget" "SnapToTarget" "SnapToTarget" true))
    (Default|SetComplete (Variables|Default|GetTrigger_Object) _returnvalue)
    (Actor|DestroyActor)))

(fn ConstructionScript)