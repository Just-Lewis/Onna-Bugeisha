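; Puzzle door that breaks apart when hit by an actor tagged YenFrag whose Trigger_Reciever reports AllComplete.
; The fragment snaps to the door's centre socket, then a timeline reveals the LazeryThings effect and two particle systems in stages.
; When the timeline ends, effects hide, attached actors detach, and an added destructible component takes radius damage as the static mesh is destroyed.
; Debug prints remain in the hit logic.
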(event EventBeginPlay
  (Variables|Default|SetStartLocation (Transformation|GetActorLocation))
  (Variables|Default|SetEmitterStartRotation (Transformation|GetWorldRotation (Variables|Default|GetLazeryThings)))
  (Rendering|SetVisibility (Variables|Default|GetParticleSystem1) false false))

(event Collision|EventHit
  (params (MyComp :type Primitive%20Component%20Object%20Reference) (Other :type Actor%20Object%20Reference) (OtherComp :type Primitive%20Component%20Object%20Reference) (bSelfMoved :type Boolean) (HitLocation :type Vector :default "0, 0, 0") (HitNormal :type Vector :default "0, 0, 0") (NormalImpulse :type Vector :default "0, 0, 0") (Hit :type Hit%20Result%20Structure%20%28by%20ref%29))
  (Development|PrintString "Hello")
  (if (Actor|ActorHasTag Other "YenFrag")
    (Development|PrintString "Is yen frag")
    (if (Variables|/Game/OB_Content/Blueprints/Functions/Trigger_Reciever.Trigger_Reciever_C|GetAllComplete (Actor|GetComponentbyClass Other "/Game/OB_Content/Blueprints/Functions/Trigger_Reciever.Trigger_Reciever_C"))
      (Transformation|AttachComponentToComponent (Variables|/Script/Engine.Actor|GetRootComponent Other) (Variables|Debug|GetStaticMeshComponent) "CentreSocket" "SnapToTarget" "SnapToTarget" "SnapToTarget" true)
      (bind _newtrack_2 (Timeline|Timeline_0 Play)
        (:Update
          (Rendering|SetVisibility (Variables|Default|GetLazeryThings) true false)
          (Rendering|SetVisibility (Variables|Default|GetParticleSystem) (> _newtrack_2 1.0) false)
          (Rendering|SetVisibility (Variables|Default|GetParticleSystem1) (> _newtrack_2 2.0) false))
        (:Finished
          (Rendering|SetVisibility (Variables|Default|GetParticleSystem1) false false)
          (bind _returnvalue (AddComponent|AddDestructibleComponent false))
          (Transformation|DetachFromActor (Actor|GetAttachedActors) "KeepRelative" "KeepRelative" "KeepRelative")
          (Rendering|ToggleVisibility (Variables|Debug|GetStaticMeshComponent) false)
          (Class|DestructibleComponent|ApplyRadiusDamage _returnvalue 1e+02 (Transformation|GetWorldLocation (Variables|Default|GetCollisionBox)) 0.0 0.0 true)
          (Components|DestroyComponent (Variables|Debug|GetStaticMeshComponent)))))
    (else
      (Development|PrintString "Is not yen frag"))))

(fn ConstructionScript)