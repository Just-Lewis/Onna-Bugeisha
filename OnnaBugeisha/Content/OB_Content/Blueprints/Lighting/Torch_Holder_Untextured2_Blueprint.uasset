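; Torch holder Blueprint that accepts a tagged actor, presumably a torch, and reports to a trigger system.
; On begin play, its TriggerObject adds itself to a set of elements.
; When an actor with the matching tag overlaps the box collider, its root component snaps to the HoldingPoint socket on the static mesh.
; The attach result is passed to TriggerObject's SetComplete.
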(event OnComponentBeginOverlap(BoxCollider)
  (params (OverlappedComponent :type Primitive%20Component%20Object%20Reference) (OtherActor :type Actor%20Object%20Reference) (OtherComp :type Primitive%20Component%20Object%20Reference) (OtherBodyIndex :type Integer) (bFromSweep :type Boolean) (SweepResult :type Hit%20Result%20Structure%20%28by%20ref%29))
  (if (Actor|ActorHasTag OtherActor (Variables|Default|GetTagToCheckFor))
    (bind _returnvalue (Transformation|AttachComponentToComponent (Variables|/Script/Engine.Actor|GetRootComponent OtherActor) (Variables|Debug|GetStaticMeshComponent) (Variables|Default|GetHoldingPoint) "SnapToTarget" "SnapToTarget" "SnapToTarget" true))
    (Default|SetComplete (Variables|Default|GetTrigger_Object) _returnvalue)))

(event EventBeginPlay
  (Default|AddtoElements (Variables|Default|GetTrigger_Object)))

(fn ConstructionScript)